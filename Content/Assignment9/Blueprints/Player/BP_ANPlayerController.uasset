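; Player controller for a number-guessing baseball game that manages the local player's UI.
; On BeginPlay it creates the main baseball widget for the local player, with cursor and game-and-UI input.
; UpdateUI events show result or error text, logging each guess and result as a record in a scroll list.
; Game end swaps in a result screen with UI-only input; clear empties the list and removes that screen.
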(event EventBeginPlay
  (if (Pawn|IsLocalPlayerController)
    (bind _returnvalue (UserInterface|CreateWidget "/Game/Assignment9/Blueprints/UI/WBP_BaseballUI.WBP_BaseballUI_C"))
    (bind _output_get (Variables|Default|SetMainUI_Ref _returnvalue))
    (UserInterface|Viewport|AddtoViewport _output_get 0)
    (Variables|Default|SetbShowMouseCursor true)
    (Input|SetInputModeGameandUI self _returnvalue "DoNotLock" true false)))

(event EventTick
  (params (DeltaSeconds :type Float%20%28single-precision%29)))

(event EventUpdateUIError
  (params (ErrorMsg :type String))
  (Rendering|Components|TextRender|SetText (Variables|/Game/Assignment9/Blueprints/UI/WBP_BaseballUI.WBP_BaseballUI_C|GetTxt_ResultBoard (Variables|Default|GetMainUI_Ref)) (Utilities|Text|ToText(String) ErrorMsg)))

(event EventUpdateUIResult
  (params (ResultMsg :type String))
  (bind _mainui_ref (Variables|Default|GetMainUI_Ref))
  (Rendering|Components|TextRender|SetText (Variables|/Game/Assignment9/Blueprints/UI/WBP_BaseballUI.WBP_BaseballUI_C|GetTxt_ResultBoard (Variables|Default|GetMainUI_Ref)) (Utilities|Text|ToText(String) ResultMsg))
  (bind _returnvalue (UserInterface|CreateWidget "/Game/Assignment9/Blueprints/UI/WBP_RecordItem.WBP_RecordItem_C"))
  (Rendering|Components|TextRender|SetText (Variables|/Game/Assignment9/Blueprints/UI/WBP_RecordItem.WBP_RecordItem_C|GetTxt_GuessedNum _returnvalue) (Variables|/Game/Assignment9/Blueprints/UI/WBP_BaseballUI.WBP_BaseballUI_C|GetLastTypedNumber _mainui_ref))
  (Rendering|Components|TextRender|SetText (Variables|/Game/Assignment9/Blueprints/UI/WBP_RecordItem.WBP_RecordItem_C|GetText_Result _returnvalue) (Utilities|Text|ToText(String) ResultMsg))
  (Widget|Panel|AddChild (Variables|/Game/Assignment9/Blueprints/UI/WBP_BaseballUI.WBP_BaseballUI_C|GetScroll_RecordList _mainui_ref) _returnvalue))

(event EventUpdateUIGameEnd
  (params (EndMsg :type String))
  (bind _mainui_ref (Variables|Default|GetMainUI_Ref))
  (Rendering|Components|TextRender|SetText (Variables|/Game/Assignment9/Blueprints/UI/WBP_BaseballUI.WBP_BaseballUI_C|GetTxt_ResultBoard _mainui_ref) (Utilities|Text|ToText(String) EndMsg))
  (Widget|RemovefromParent _mainui_ref)
  (bind _returnvalue (UserInterface|CreateWidget "/Game/Assignment9/Blueprints/UI/WBP_Result.WBP_Result_C"))
  (Rendering|Components|TextRender|SetText (Variables|/Game/Assignment9/Blueprints/UI/WBP_Result.WBP_Result_C|GetTxt_ResultTitle _returnvalue) (Utilities|Text|ToText(String) EndMsg))
  (UserInterface|Viewport|AddtoViewport _returnvalue 0)
  (Input|SetInputModeUIOnly (Game|GetPlayerController 0) _returnvalue "DoNotLock" false)
  (Variables|Default|SetbShowMouseCursor true))

(event EventUpdateUIClear
  (Widget|Panel|ClearChildren (Variables|/Game/Assignment9/Blueprints/UI/WBP_BaseballUI.WBP_BaseballUI_C|GetScroll_RecordList (Variables|Default|GetMainUI_Ref)))
  (Widget|RemovefromParent (stale EventUpdateUIGameEnd _returnvalue)))

(fn ConstructionScript)